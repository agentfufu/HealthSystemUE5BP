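; BP_Trap is a trap that repeatedly damages an actor while it overlaps the trap's Collision component.
; Begin overlap stores the most recent overlapping actor, sets IsOverlapping and starts TakeDamage, which sends TakeDamageMessage with Damage to that actor.
; TakeDamage then calls itself after a WaitingTime delay, looping until any end overlap clears the flag.
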(event `self.Collision.OnComponentBeginOverlap`
  (params (OverlappedComponent :type "PrimitiveComponent Object Reference") (OtherActor :type "Actor Object Reference") (OtherComp :type "PrimitiveComponent Object Reference") (OtherBodyIndex :type Integer) (bFromSweep :type Boolean) (SweepResult :type "HitResult Structure (by ref)"))
  ;[1 1 1] When BeginOverlap the trap , we call the event take damage and set IsOverlapping to True
  (set `self.IsOverlapping?` true)
  (set `self.Overlaping Actor` OtherActor)
  (`self.TakeDamage`))

(event `TakeDamage`
  ;[1 1 1] Verify if we are overlapping , if yes , Send a event to Overlaping actor , Then wait and damage again in case still overlapping.
  (if (`self.IsOverlapping?`)
    (message `/Game/Health/BPI_Health.Take Damage` (`self.Overlaping Actor`) (`self.Damage`))
    (`KismetSystemLibrary.Delay` (`self.WaitingTime`))
    (`self.TakeDamage`)))

(event `self.Collision.OnComponentEndOverlap`
  (params (OverlappedComponent :type "PrimitiveComponent Object Reference") (OtherActor :type "Actor Object Reference") (OtherComp :type "PrimitiveComponent Object Reference") (OtherBodyIndex :type Integer))
  ;[1 1 1] Turn Overlapping Off
  (set `self.IsOverlapping?` false))

(fn `UserConstructionScript`)