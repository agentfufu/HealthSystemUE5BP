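; Health pickup actor that repeatedly heals whatever actor stands inside its box trigger.
; Begin overlap stores that single actor and starts Heal, which sends it the heal amount through an interface message and re-calls itself after a very short delay until any end overlap clears the flag.
; Tick spins the medkit component by a fixed yaw step each frame, unscaled by delta time.
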(event `Heal`
  ;[1 1 1] Check if the actor is overlapping , if true, send Heal Event to the overlapping actor , then wait and check if still overlapping , also send the Heal Amount
  (if (`self.IsOverlapping?`)
    (message `/Game/Health/BPI_Health.Heal` (`self.OverlappingActor`) (`self.HealAmount`))
    (`KismetSystemLibrary.Delay` 0.01)
    (`self.Heal`)))

(event `self.Box.OnComponentBeginOverlap`
  (params (OverlappedComponent :type "PrimitiveComponent Object Reference") (OtherActor :type "Actor Object Reference") (OtherComp :type "PrimitiveComponent Object Reference") (OtherBodyIndex :type Integer) (bFromSweep :type Boolean) (SweepResult :type "HitResult Structure (by ref)"))
  ;[1 1 1] Begin Overlap and put the overlapping actor into a variable,then call the custom event Heal
  (set `self.IsOverlapping?` true)
  (set `self.OverlappingActor` OtherActor)
  (`self.Heal`))

(event `self.Box.OnComponentEndOverlap`
  (params (OverlappedComponent :type "PrimitiveComponent Object Reference") (OtherActor :type "Actor Object Reference") (OtherComp :type "PrimitiveComponent Object Reference") (OtherBodyIndex :type Integer))
  (set `self.IsOverlapping?` false))

(event `self.ReceiveTick`
  (params (DeltaSeconds :type "Float (single-precision)"))
  (`SceneComponent.K2_AddRelativeRotation` (`self.old_medkits`) (`KismetMathLibrary.MakeRotator` 0.0 0.0 500.0) false false))

(fn `UserConstructionScript`)